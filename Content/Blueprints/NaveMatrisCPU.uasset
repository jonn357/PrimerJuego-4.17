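; CPU-controlled mothership (NaveMatris) that drifts along negative X, fires bullets and can be destroyed.
; A looping timer calls disparo, which spawns a Bala at the actor's Y and Z but half its world X.
; Overlaps with components tagged as ships or player bullets subtract health and set SinVida at zero or below.
; Tick moves the static mesh and destroys the actor once that flag is set.
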(event OnComponentBeginOverlap(StaticMeshComponent)
  (params (OverlappedComponent :type Primitive%20Component%20Object%20Reference) (OtherActor :type Actor%20Object%20Reference) (OtherComp :type Primitive%20Component%20Object%20Reference) (OtherBodyIndex :type Integer) (bFromSweep :type Boolean) (SweepResult :type Hit%20Result%20Structure%20%28by%20ref%29))
  (if (Math|Boolean|ORBoolean (Components|ComponentHasTag OtherComp "NaveCaza") (Components|ComponentHasTag OtherComp "NaveMatris") (Components|ComponentHasTag OtherComp "NavePrincipal") (Components|ComponentHasTag OtherComp "BalaPlayer"))
    (bind _output_get (Variables|Default|SetvidaNaveMatrisCPU (+ -10 (Variables|Default|GetvidaNaveMatrisCPU))))
    (if (<= _output_get 0)
      (Variables|Default|SetsinVida true))))

(event Custom|disparo
  (bind _returnvalue (Transformation|GetActorLocation))
  (bind (_x _y _z) (Math|Vector|BreakVector _returnvalue))
  (Game|SpawnActorfromClass "/Game/Blueprints/bala.bala_C" (Math|Transform|MakeTransform (Math|Vector|MakeVector (* _x 0.5) _y _z) "0, 0,0.000000" "1.000000,1,1") "Undefined" 0 0))

(event EventBeginPlay
  (Utilities|Time|SetTimerbyFunctionName 0 "disparo" 2.0 true))

(event Collision|EventActorBeginOverlap
  (params (OtherActor :type Actor%20Object%20Reference)))

(event EventTick
  (params (DeltaSeconds :type Float%20%28single-precision%29))
  (Transformation|AddRelativeLocation (Variables|Debug|GetStaticMeshComponent) (* "-100.000000,0.000000,0.000000" DeltaSeconds) false false)
  (if (Variables|Default|GetsinVida)
    (Actor|DestroyActor)))

(fn ConstructionScript)