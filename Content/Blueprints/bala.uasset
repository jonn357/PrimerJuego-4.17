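; Bala is a projectile actor, apparently fired by CPU ships, that moves its static mesh along negative relative X at constant speed.
; Overlaps with components tagged as player bullets or ships reduce its health variable, VidaNaveCazaCPU, and set SinVida once it runs out.
; Tick destroys the actor when SinVida is set or when a frame-counted lifetime expires, so lifespan depends on frame rate.
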(event OnComponentBeginOverlap(StaticMeshComponent)
  (params (OverlappedComponent :type Primitive%20Component%20Object%20Reference) (OtherActor :type Actor%20Object%20Reference) (OtherComp :type Primitive%20Component%20Object%20Reference) (OtherBodyIndex :type Integer) (bFromSweep :type Boolean) (SweepResult :type Hit%20Result%20Structure%20%28by%20ref%29))
  ;[1 1 1] recivir daño
  (if (Math|Boolean|ORBoolean (Components|ComponentHasTag OtherComp "BalaPlayer") (Components|ComponentHasTag OtherComp "NavePrincipal") (Components|ComponentHasTag OtherComp "NaveCaza") (Components|ComponentHasTag OtherComp "NaveMatris"))
    (bind _output_get (Variables|Default|SetvidaNaveCazaCPU (+ (Variables|Default|GetvidaNaveCazaCPU) -10)))
    (if (<= _output_get 0)
      (Variables|Default|SetsinVida true))))

(event EventBeginPlay)

(event Collision|EventActorBeginOverlap
  (params (OtherActor :type Actor%20Object%20Reference)))

(event EventTick
  (params (DeltaSeconds :type Float%20%28single-precision%29))
  ;[1 1 1] Desplaza la Nave
  (Variables|Default|Settimer (+ 1 (Variables|Default|Gettimer)))
  (Transformation|AddRelativeLocation (Variables|Debug|GetStaticMeshComponent) (* "-300.000000, 0, 0" DeltaSeconds) false false)
  (if (Variables|Default|GetsinVida)
    (Actor|DestroyActor :!label _label)
    (elif (> (Variables|Default|GetTimer) 500)
      (goto _label))))

(fn ConstructionScript)