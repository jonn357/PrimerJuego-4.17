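; NavePrincipal is a ship actor that moves itself and fires BalaPlayer bullets.
; Each Tick increments Timer, offsets the mesh by cosine and sine expressions scaled by Velocidad, and spawns a bullet at the actor's location.
; Tick destroys the actor when SinVida is true, but the tag-based damage logic that sets it is disconnected from the empty overlap event, so it never runs.
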(event OnComponentBeginOverlap(StaticMeshComponent)
  (params (OverlappedComponent :type Primitive%20Component%20Object%20Reference) (OtherActor :type Actor%20Object%20Reference) (OtherComp :type Primitive%20Component%20Object%20Reference) (OtherBodyIndex :type Integer) (bFromSweep :type Boolean) (SweepResult :type Hit%20Result%20Structure%20%28by%20ref%29)))

(event EventBeginPlay)

(event EventTick
  (params (DeltaSeconds :type Float%20%28single-precision%29))
  (Variables|Default|Settimer (+ 1 (Variables|Default|Gettimer)))
  (Transformation|AddRelativeLocation (Variables|Debug|GetStaticMeshComponent) (* (Math|Vector|MakeVector (|({D2A81215-4D0C-5BAE-02A0-C09448C2496A}+({38F2DD5F-4F9C-0CC7-64A2-C49C93763010}*(cos({157408E3-41B1-4C0D-AC69-D199D7221C08}))))) (|({2E6C2C74-4606-6B43-6E44-D8A136AE6464}+({F8B057CA-4E89-67A2-F975-BE9393159856}*(sin({157408E3-41B1-4C0D-AC69-D199D7221C08}))))) 0.0) (Variables|Default|Getvelocidad)) false false)
  (Game|SpawnActorfromClass "/Game/Blueprints/BalaPlayer.BalaPlayer_C" (Math|Transform|MakeTransform (Transformation|GetActorLocation) "0, 0,0.000000" "1.000000,1,1") "Undefined" 0 0)
  (if (Variables|Default|GetsinVida)
    (Actor|DestroyActor)))

(fn ConstructionScript)