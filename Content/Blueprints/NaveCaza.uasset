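; NaveCaza is a fighter ship Blueprint that tracks its own health and destroys itself when that health runs out.
; Overlaps on its static mesh with components tagged as a bullet (Bala), CPU fighter, CPU mothership or main ship reduce VidaNaveCaza by a fixed amount.
; At zero health or below it sets the SinVida flag, which Tick polls every frame to call DestroyActor.
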(event OnComponentBeginOverlap(StaticMeshComponent)
  (params (OverlappedComponent :type Primitive%20Component%20Object%20Reference) (OtherActor :type Actor%20Object%20Reference) (OtherComp :type Primitive%20Component%20Object%20Reference) (OtherBodyIndex :type Integer) (bFromSweep :type Boolean) (SweepResult :type Hit%20Result%20Structure%20%28by%20ref%29))
  (if (Math|Boolean|ORBoolean (Components|ComponentHasTag OtherComp "Bala") (Components|ComponentHasTag OtherComp "NaveCazaCPU") (Components|ComponentHasTag OtherComp "NaveMatrisCPU") (Components|ComponentHasTag OtherComp "NavePrincipal"))
    (bind _output_get (Variables|Default|SetvidaNaveCaza (+ (Variables|Default|GetvidaNaveCaza) -10)))
    (if (<= _output_get 0)
      (Variables|Default|SetsinVida true))))

(event EventBeginPlay)

(event Collision|EventActorBeginOverlap
  (params (OtherActor :type Actor%20Object%20Reference)))

(event EventTick
  (params (DeltaSeconds :type Float%20%28single-precision%29))
  (if (Variables|Default|GetsinVida)
    (Actor|DestroyActor)))

(fn ConstructionScript)