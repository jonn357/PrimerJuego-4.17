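; NaveMatris is a player-controlled ship that moves, fires and takes damage.
; Arrow keys and Touch1 set persistent axis speeds that Tick applies as a relative offset without sweep, so it keeps moving after release.
; PageUp spawns a BalaPlayer at the ship's location.
; Overlaps with components tagged as bullets or CPU ships reduce health, and at zero a flag makes Tick destroy the actor.
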(event OnComponentBeginOverlap(naveMatris)
  (params (OverlappedComponent :type Primitive%20Component%20Object%20Reference) (OtherActor :type Actor%20Object%20Reference) (OtherComp :type Primitive%20Component%20Object%20Reference) (OtherBodyIndex :type Integer) (bFromSweep :type Boolean) (SweepResult :type Hit%20Result%20Structure%20%28by%20ref%29))
  (if (Math|Boolean|ORBoolean (Components|ComponentHasTag OtherComp "Bala") (Components|ComponentHasTag OtherComp "NaveMatrisCPU") (Components|ComponentHasTag OtherComp "NaveCazaCPU"))
    (bind _output_get (Variables|Default|SetvidaNaveMatris (+ (Variables|Default|GetvidaNaveMatris) -10)))
    (if (<= _output_get 0)
      (Variables|Default|SetsinVida true))))

(event EventTick
  (params (DeltaSeconds :type Float%20%28single-precision%29))
  (Transformation|AddRelativeLocation (Variables|Default|GetnaveMatris) (* (Math|Vector|MakeVector (Variables|Default|Getabajo) (Variables|Default|Getarriba) 0.0) DeltaSeconds) false false)
  (if (Variables|Default|GetsinVida)
    (Actor|DestroyActor)))

(event Input|KeyboardEvents|PageUp
  (params (Key :type Key%20Structure :default "AnyKey"))
  (:Pressed
    (Game|SpawnActorfromClass "/Game/Blueprints/BalaPlayer.BalaPlayer_C" (Math|Transform|MakeTransform (Transformation|GetActorLocation) "0, 0, 0" "1,1,1") "Undefined" 0 0)))

(event Input|TouchEvents|Touch1
  (params (Key :type Key%20Structure :default "AnyKey"))
  ;[1 1 1] Inputs
  (:Pressed
    (Variables|Default|Setarriba -2e+02)))

(event Input|KeyboardEvents|Up
  (params (Key :type Key%20Structure :default "AnyKey"))
  ;[1 1 1] Inputs
  (:Pressed
    (Variables|Default|Setarriba -2e+02)))

(event Input|KeyboardEvents|Down
  (params (Key :type Key%20Structure :default "AnyKey"))
  ;[1 1 1] Inputs
  (:Pressed
    (Variables|Default|Setarriba 2e+02)))

(event Input|KeyboardEvents|Left
  (params (Key :type Key%20Structure :default "AnyKey"))
  ;[1 1 1] Inputs
  (:Pressed
    (Variables|Default|Setabajo -2e+02)))

(event Input|KeyboardEvents|Right
  (params (Key :type Key%20Structure :default "AnyKey"))
  ;[1 1 1] Inputs
  (:Pressed
    (Variables|Default|Setabajo 2e+02)))

(fn ConstructionScript)