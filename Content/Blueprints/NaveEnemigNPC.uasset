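; NaveEnemigNPC is an enemy ship that drifts along negative X, fires Bala projectiles and spawns copies of itself on looping timers.
; BeginPlay starts both timers and updates the HUD through HUD_Control.
; Overlaps with components tagged as player ships or player bullets drain its health until SinVida is set.
; Tick then increments Score on the naveMatris reference, whose assignment here is unwired, and destroys the ship.
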(event OnComponentBeginOverlap(NaveEnemigaNPC)
  (params (OverlappedComponent :type Primitive%20Component%20Object%20Reference) (OtherActor :type Actor%20Object%20Reference) (OtherComp :type Primitive%20Component%20Object%20Reference) (OtherBodyIndex :type Integer) (bFromSweep :type Boolean) (SweepResult :type Hit%20Result%20Structure%20%28by%20ref%29))
  (if (Math|Boolean|ORBoolean (Components|ComponentHasTag OtherComp "NaveCaza") (Components|ComponentHasTag OtherComp "NaveMatris") (Components|ComponentHasTag OtherComp "NavePrincipal") (Components|ComponentHasTag OtherComp "BalaPlayer_BP"))
    (bind _output_get (Variables|Default|SetvidaNaveMatrisCPU (+ -10 (Variables|Default|GetvidaNaveMatrisCPU))))
    (if (<= _output_get 0)
      (Variables|Default|SetsinVida true))))

(event Custom|FuncionDesove
  (Game|SpawnActorfromClass "NaveEnemigNPC_C" (Math|Transform|MakeTransform (Transformation|GetActorLocation) "0, 0, 0" "1,1,1") "Undefined" 0 0 0 0))

(event Custom|disparo
  (bind _returnvalue (Transformation|GetActorLocation))
  (bind (_x _y _z) (Math|Vector|BreakVector _returnvalue))
  (Game|SpawnActorfromClass "/Game/Blueprints/bala.bala_C" (Math|Transform|MakeTransform (Math|Vector|MakeVector (* _x 0.5) _y _z) "0.000000,0.000000,0.000000" "1.000000,1.000000,1.000000") "Undefined" 0 0))

(event EventTick
  (params (DeltaSeconds :type Float%20%28single-precision%29))
  (Transformation|AddRelativeLocation (Variables|Default|GetNaveEnemigaNPC) (* "-100.000000,0.000000,0.000000" DeltaSeconds) false false)
  (if (Variables|Default|GetsinVida)
    ;[1 1 1] Contar # de Naves Destruidas
    (bind _asnave_matris (Utilities|Casting|CastTonaveMatris (Variables|Default|GetRefNaveMatris))
      (:then
        _)
      (:CastFailed
        _))
    (Variables|/Game/Blueprints/naveMatris.naveMatris_C|SetScore _asnave_matris (+ (Variables|/Game/Blueprints/naveMatris.naveMatris_C|GetScore _asnave_matris) 1))
    (Actor|DestroyActor)))

(event EventBeginPlay
  (Utilities|Time|SetTimerbyFunctionName 0 "disparo" 2.0 true)
  (Utilities|Time|SetTimerbyFunctionName 0 "FuncionDesove" 5.0 true)
  (bind _ashud_control (Utilities|Casting|CastToHUD_Control (HUD|GetHUD (Game|GetPlayerController 0))))
  ;[1 1 1] Crear Referencia a HUD Control
  (Default|ActualizarScort (Variables|/Game/UI/HUD_Control.HUD_Control_C|GetHUD _ashud_control) 1))

(fn ConstructionScript)