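; BalaPlayer_BP is the player's bullet, a projectile that flies forward and has its own health.
; Tick moves the StaticMesh along local X by a frame-rate-dependent step scaled by Velocidad, and destroys the actor when SinVida is set or a frame-count lifetime expires.
; Overlaps with actors tagged Bala or NaveCazaCPU reduce VidaBalaPlayer, setting SinVida at zero.
; EnviarReferencia stores a passed actor reference, unused within these graphs.
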(event OnComponentBeginOverlap(StaticMesh)
  (params (OverlappedComponent :type Primitive%20Component%20Object%20Reference) (OtherActor :type Actor%20Object%20Reference) (OtherComp :type Primitive%20Component%20Object%20Reference) (OtherBodyIndex :type Integer) (bFromSweep :type Boolean) (SweepResult :type Hit%20Result%20Structure%20%28by%20ref%29))
  ;[1 1 1] recivir daño
  (if (or (Components|ComponentHasTag OtherComp "Bala") (Components|ComponentHasTag OtherComp "NaveCazaCPU"))
    (bind _output_get (Variables|Default|SetVidaBalaPlayer (+ (Variables|Default|GetVidaBalaPlayer) -10)))
    (if (<= _output_get 0)
      (Variables|Default|SetsinVida true))))

(event EventTick
  (params (DeltaSeconds :type Float%20%28single-precision%29))
  ;[1 1 1] Desplaza la Nave
  (Variables|Default|SetTimer (+ 1 (Variables|Default|GetTimer)))
  (Transformation|AddRelativeLocation (Variables|Default|GetStaticMesh) (* (- "50.000000, 0, 0" DeltaSeconds) (Variables|Default|Getvelocidad)) false false)
  (if (Variables|Default|GetsinVida)
    (Actor|DestroyActor :!label _label)
    (elif (> (Variables|Default|GetTimer) 70)
      (goto _label))))

(fn ConstructionScript)

(fn EnviarReferencia
  (params (Actor1 :type Actor%20Object%20Reference))
  (Variables|Default|Setreferencia1 Actor1))